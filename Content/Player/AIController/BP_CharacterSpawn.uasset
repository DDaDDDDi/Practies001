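; Trigger actor that spawns a BP_CPlayer_Warrior character when a BP_CPlayer overlaps it.
; BeginPlay sets the class to spawn, and the overlap spawns it at the overlapping player's location offset by Target.
; The spawned actor is stored in Characters, so another spawns only once that reference is no longer valid.
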(event EventBeginPlay
  (Variables|Default|SetCharacterClass "/Game/Player/BP_CPlayer_Warrior.BP_CPlayer_Warrior_C"))

(event Collision|EventActorBeginOverlap
  (params (OtherActor :type Actor%20Object%20Reference))
  (Utilities|Casting|CastToBP_CPlayer OtherActor)
  (Utilities|IsValid (Variables|Default|GetCharacters)
    (:Is%20Not%20Valid
      (bind _returnvalue (Game|SpawnActorfromClass (Variables|Default|GetCharacterClass) (Math|Conversions|ToTransform(Vector) (+ (Transformation|GetActorLocation OtherActor) (Variables|Default|GetTarget))) "Undefined" 0 0))
      (Variables|Default|SetCharacters _returnvalue))))

(event EventTick
  (params (DeltaSeconds :type Float%20%28single-precision%29)))

(fn ConstructionScript)