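; Enemy spawn trigger that spawns copies of the actors in its Enemies array when any actor overlaps it.
; For each valid enemy, it spawns that actor's class at every Target transform, using location as an offset from the trigger and ignoring scale.
; A Stack counter increments up to four but does not limit spawning, as both branches spawn identically.
; Each spawn overwrites Enemies with the two branches' latest spawned actors.
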(event EventBeginPlay)

(event Collision|EventActorBeginOverlap
  (params (OtherActor :type Actor%20Object%20Reference))
  (bind _output_get (Variables|Default|SetEnemies (Variables|Default|GetEnemies)))
  (bind _array_element (Utilities|Array|ForEachLoopwithBreak _output_get)
    (:LoopBody
      (for _array_element_2 (Variables|Default|GetTarget)
        (Utilities|IsValid _array_element
          (:Is%20Valid
            (if (> (Variables|Default|GetStack) 3)
              (bind _returnvalue (Game|SpawnActorfromClass (Utilities|GetClass _array_element) (Math|Transform|MakeTransform (+ (Transformation|GetActorLocation) (.Location (Math|Transform|BreakTransform _array_element_2))) (.Rotation (Math|Transform|BreakTransform _array_element_2))) "Undefined" 0 0))
              (else
                (bind _returnvalue_2 (Game|SpawnActorfromClass (Utilities|GetClass _array_element) (Math|Transform|MakeTransform (+ (Transformation|GetActorLocation) (.Location (Math|Transform|BreakTransform _array_element_2))) (.Rotation (Math|Transform|BreakTransform _array_element_2))) "Undefined" 0 0))
                (Math|Integer|IncrementInt (Variables|Default|GetStack)
                  (:%20%20
                    _))))
            (Variables|Default|SetEnemies (Utilities|Array|MakeArray _returnvalue_2 _returnvalue))))))))

(event EventTick
  (params (DeltaSeconds :type Float%20%28single-precision%29)))

(fn ConstructionScript)